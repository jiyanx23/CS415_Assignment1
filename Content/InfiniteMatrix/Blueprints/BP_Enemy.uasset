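; BP_Enemy is an enemy actor that awards score when shot and damages the player on contact, with all logic in its static mesh's begin-overlap event.
; A projectile overlap adds points to that projectile's owning player through Score and ChangeScore, then destroys the enemy.
; A player overlap shakes the camera and subtracts health.
; The enemy destroys itself on contact only when health hits exactly zero, also marking the player dead and showing restart.
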(event `self.StaticMesh.OnComponentBeginOverlap`
  (params (OverlappedComponent :type "PrimitiveComponent Object Reference") (OtherActor :type "Actor Object Reference") (OtherComp :type "PrimitiveComponent Object Reference") (OtherBodyIndex :type Integer) (bFromSweep :type Boolean) (SweepResult :type "HitResult Structure (by ref)"))
  (`|ExecutionSequence`
    (:`then_0`
      (bind _asbp_projectile (cast `/Game/InfiniteMatrix/Blueprints/BP_Projectile` OtherActor))
      (bind _player (`/Game/InfiniteMatrix/Blueprints/BP_Projectile.player` _asbp_projectile))
      (bind _output_get (set `/Game/InfiniteMatrix/Blueprints/BP_Player.Score` (+ (`/Game/InfiniteMatrix/Blueprints/BP_Player.ChangeScore` _player) 20) _player))
      (set `/Game/InfiniteMatrix/Blueprints/BP_Player.ChangeScore` _output_get _player)
      (`self.K2_DestroyActor`))
    (:`then_1`
      (bind _asbp_player (cast `/Game/InfiniteMatrix/Blueprints/BP_Player` OtherActor))
      (`MatineeCameraShake.StartMatineeCameraShake` (`GameplayStatics.GetPlayerCameraManager` 0) "/Game/InfiniteMatrix/Blueprints/BP_CameraShake.BP_CameraShake_C")
      (bind _output_get_2 (set `/Game/InfiniteMatrix/Blueprints/BP_Player.CurrentHealth` (- (`/Game/InfiniteMatrix/Blueprints/BP_Player.CurrentHealth` _asbp_player) 20.0) _asbp_player))
      (if (== _output_get_2 0.0)
        (set `/Game/InfiniteMatrix/Blueprints/BP_Player.IsDead` true _asbp_player)
        (`/Game/InfiniteMatrix/Blueprints/BP_Player.DisplayRestart` _asbp_player)
        (`self.K2_DestroyActor`)))))

(fn `UserConstructionScript`)