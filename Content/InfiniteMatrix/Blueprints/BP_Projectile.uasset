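; BP_Projectile is a projectile that destroys itself on hitting an enemy or the tunnel.
; The construction script copies ProjectileSpeed into the ProjectileMovement component's initial speed.
; Sphere overlaps ignore BP_Player and set ShouldDisappear for BP_Enemy or BP_Tunnel, and Tick then destroys the actor.
; It applies no damage itself, and a leftover time-based despawn check is disconnected and never runs.
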(event `self.ReceiveBeginPlay`)

(event `self.ReceiveTick`
  (params (DeltaSeconds :type "Float (single-precision)"))
  (if (`self.shouldDisappear`)
    (`self.K2_DestroyActor`)))

(event `self.Sphere.OnComponentBeginOverlap`
  (params (OverlappedComponent :type "PrimitiveComponent Object Reference") (OtherActor :type "Actor Object Reference") (OtherComp :type "PrimitiveComponent Object Reference") (OtherBodyIndex :type Integer) (bFromSweep :type Boolean) (SweepResult :type "HitResult Structure (by ref)"))
  (cast `/Game/InfiniteMatrix/Blueprints/BP_Player` OtherActor
    (:`CastFailed`
      (`|ExecutionSequence`
        (:`then_0`
          (cast `/Game/InfiniteMatrix/Blueprints/BP_Enemy` OtherActor
            (:`then`
              (set `self.shouldDisappear` true))
            (:`CastFailed`
              (cast `/Game/InfiniteMatrix/Blueprints/BP_Tunnel` OtherActor)
              (set `self.shouldDisappear` true))))))))

(fn `SetInitialProjectileSpeed`
  (set `ProjectileMovementComponent.InitialSpeed` (`self.projectileSpeed`) (`self.ProjectileMovement`)))

(fn `UserConstructionScript`
  (`self.SetInitialProjectileSpeed`))